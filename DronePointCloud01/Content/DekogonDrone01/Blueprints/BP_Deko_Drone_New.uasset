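; Player-flown drone pawn with toggleable ignition, switched on at BeginPlay.
; Enhanced Input values feed Tick, which adds yaw-relative velocity to the physics body and interpolates tilt and stepped mouse yaw; engine-off zeroes control and adds descent.
; Tick also drives engine audio from speed and spins propellers up or down through the Anim Blueprint, while look-up pitches the spring arm.
; Construction script selects the turret mesh and applies material, color and emissive settings.
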(event `self.ReceiveBeginPlay`
  ;[1 1 1] Beginplay
  (`|ExecutionSequence`
    (:`then_0`
      (bind _asplayer_controller (cast `PlayerController` (`self.GetController`)))
      (bind _returnvalue (pcsubsystem `EnhancedInputLocalPlayerSubsystem` _asplayer_controller))
      (`/Engine/EditorBlueprintResources/StandardMacros.IsValid` _returnvalue
        (:`Is Valid`
          (`EnhancedInputSubsystemInterface.AddMappingContext` _returnvalue "/Game/DekogonDrone01/Blueprints/Input/IMC_Default.IMC_Default" 0 (struct))
          (`self.K2_AddActorWorldOffset` (0.0 0.0 50.0))
          (`self.IgniteOnStart`))))
    (:`then_1`
      (bind _asabp_deko_drone_01a (cast `/Game/DekogonDrone01/Blueprints/ABP_Deko_Drone_01a` (`SkeletalMeshComponent.GetAnimInstance` (`self.DekogonDrone`))))
      (set `self.DEKODRONEABP` _asabp_deko_drone_01a))))

(event `IgniteOnStart`
  ;[1 1 1] Ignition
  (bind _isa (`/Engine/EditorBlueprintResources/StandardMacros.FlipFlop` :!label _label)
    (:`A`
      _)
    (:`B`
      _))
  (set `self.Start Awake` _isa))

(event `EnhancedInput|/Game/DekogonDrone01/Blueprints/Input/IA_Ignition`
  (params (ActionValue :type Boolean) (ElapsedSeconds :type "Float (double-precision)") (TriggeredSeconds :type "Float (double-precision)") (InputAction :type "InputAction Object Reference" :default "/Game/DekogonDrone01/Blueprints/Input/IA_Ignition.IA_Ignition"))
  ;[1 1 1] Ignition
  (:`Started`
    (goto _label)))

(event `EnhancedInput|/Game/DekogonDrone01/Blueprints/Input/IA_Throttle`
  (params (ActionValue :type "Float (double-precision)") (ElapsedSeconds :type "Float (double-precision)") (TriggeredSeconds :type "Float (double-precision)") (InputAction :type "InputAction Object Reference" :default "/Game/DekogonDrone01/Blueprints/Input/IA_Throttle.IA_Throttle"))
  ;[1 1 1] Analogs
  (:`Triggered`
    (set `self.Throttle` ActionValue :!label _label_2))
  (:`Started`
    (goto _label_2))
  (:`Completed`
    (goto _label_2)))

(event `self.ReceiveTick`
  (params (DeltaSeconds :type "Float (single-precision)"))
  (bind (_returnvalue_roll _returnvalue_pitch _returnvalue_yaw) (`KismetMathLibrary.BreakRotator` (`self.K2_GetActorRotation`)))
  (bind (_returnvalue_roll_2 _returnvalue_pitch_2 _returnvalue_yaw_2) (`KismetMathLibrary.BreakRotator` (`self.K2_GetActorRotation`)))
  (bind _propellerspeed (`self.PropellerSpeed`))
  (bind _delta_seconds (`self.Delta seconds`))
  (bind _sc_dekodrone_engine (`self.SC_DekoDrone_Engine`))
  (bind _start_awake (`self.Start Awake`))
  (bind _dekodroneabp (`self.DEKODRONEABP`))
  (bind _returnvalue (`KismetMathLibrary.Conv_BoolToDouble` _start_awake))
  (bind _returnvalue_2 (`KismetMathLibrary.Conv_BoolToDouble` (`self.Start Awake`)))
  (bind _returnvalue_3 (* _delta_seconds (`self.PropellerAcceleration`)))
  (bind _returnvalue_4 (`KismetMathLibrary.FClamp` (- _propellerspeed _returnvalue_3) 0.0 (`self.MaxPropellerSpeed`)))
  (bind _returnvalue_5 (`KismetMathLibrary.FClamp` (+ _propellerspeed _returnvalue_3) 0.0 (`self.MaxPropellerSpeed`)))
  (bind _returnvalue_6 (`KismetMathLibrary.FInterpTo` (`self.SoundSpeed`) (`KismetMathLibrary.SelectFloat` (`KismetMathLibrary.Abs` (`KismetMathLibrary.VSize` (`self.GetVelocity`))) -6.0 (`self.Start Awake`)) (`self.Delta seconds`) 50.0))
  (bind (_returnvalue_roll_3 _returnvalue_pitch_3) (`KismetMathLibrary.BreakRotator` (`KismetMathLibrary.MakeRotator` (+ (* (`self.MouseRot`) 5.0 _returnvalue_2) (* (`self.Steer`) 25.0 _returnvalue_2)) (+ (* (`self.Throttle`) -25.0 _returnvalue_2) (* (`self.Up`) 10.0 _returnvalue_2)))))
  (bind (_returnvalue_roll_4 _returnvalue_pitch_4 _returnvalue_yaw_3) (`KismetMathLibrary.BreakRotator` (`KismetMathLibrary.RInterpTo` (`KismetMathLibrary.MakeRotator` _returnvalue_roll _returnvalue_pitch _returnvalue_yaw) (`KismetMathLibrary.MakeRotator` _returnvalue_roll_3 _returnvalue_pitch_3 (+ _returnvalue_yaw (* (`self.MouseRot`) (`self.Drone Horizontal Rotation`) _returnvalue_2))) (`self.Delta seconds`) 1.0)))
  ;[1 1 1] DroneMovement
  (set `self.Delta seconds` DeltaSeconds)
  (`PrimitiveComponent.SetPhysicsLinearVelocity` (`self.PhysicsObject`) (+ (`self.GetVelocity`) (* (* (`KismetMathLibrary.GreaterGreater_VectorRotator` (`KismetMathLibrary.MakeVector` (* (`self.Throttle`) _returnvalue) (* _returnvalue (`self.Steer`)) (`KismetMathLibrary.SelectFloat` (`self.Up`) -1.0 _start_awake)) (`KismetMathLibrary.MakeRotator` 0.0 0.0 _returnvalue_yaw_2)) (`self.Movement speed`)) (`self.Delta seconds`))) false "None")
  (`self.K2_SetActorRotation` (`KismetMathLibrary.MakeRotator` _returnvalue_roll_4 _returnvalue_pitch_4 _returnvalue_yaw_3)) ; Rotate the helicopter yaw to match the camera, while pitch and roll are determined by input direction
  ;[1 1 1] Audio&Animation
  (bind _output_get (set `self.SoundSpeed` _returnvalue_6))
  (`AudioComponent.SetFloatParameter` _sc_dekodrone_engine "Throttle" _output_get)
  (`AudioComponent.SetPitchMultiplier` _sc_dekodrone_engine (* (+ (/ _returnvalue_6 9000.0) 0.2) 3.0))
  (if (`self.Start Awake`)
    (set `self.PropellerSpeed` _returnvalue_5) ; Rotation coefficient
    (set `self.CurrentPropellerRot` (`KismetMathLibrary.ClampAxis` (+ (`self.CurrentPropellerRot`) (* _delta_seconds _returnvalue_5))))
    (else
      (set `self.PropellerSpeed` _returnvalue_4) ; Rotation coefficient
      (bind _output_get_2 (set `self.CurrentPropellerRot` (`KismetMathLibrary.ClampAxis` (+ (`self.CurrentPropellerRot`) (* _delta_seconds _returnvalue_4)))))))
  (bind _output_get_3 (set `/Game/DekogonDrone01/Blueprints/ABP_Deko_Drone_01a.FL_Propeller` _output_get_2 _dekodroneabp))
  (bind _output_get_4 (set `/Game/DekogonDrone01/Blueprints/ABP_Deko_Drone_01a.BL_Propeller` _output_get_3 _dekodroneabp))
  (bind _output_get_5 (set `/Game/DekogonDrone01/Blueprints/ABP_Deko_Drone_01a.BR_Propeller` _output_get_4 _dekodroneabp))
  (set `/Game/DekogonDrone01/Blueprints/ABP_Deko_Drone_01a.FR_Propeller` _output_get_5 _dekodroneabp))

(event `EnhancedInput|/Game/DekogonDrone01/Blueprints/Input/IA_Steer`
  (params (ActionValue :type "Float (double-precision)") (ElapsedSeconds :type "Float (double-precision)") (TriggeredSeconds :type "Float (double-precision)") (InputAction :type "InputAction Object Reference" :default "/Game/DekogonDrone01/Blueprints/Input/IA_Steer.IA_Steer"))
  ;[1 1 1] Analogs
  (:`Triggered`
    (set `self.Steer` ActionValue :!label _label_3))
  (:`Started`
    (goto _label_3))
  (:`Completed`
    (goto _label_3)))

(event `EnhancedInput|/Game/DekogonDrone01/Blueprints/Input/IA_Up`
  (params (ActionValue :type "Float (double-precision)") (ElapsedSeconds :type "Float (double-precision)") (TriggeredSeconds :type "Float (double-precision)") (InputAction :type "InputAction Object Reference" :default "/Game/DekogonDrone01/Blueprints/Input/IA_Up.IA_Up"))
  ;[1 1 1] Analogs
  (:`Triggered`
    (set `self.Up` ActionValue :!label _label_4))
  (:`Started`
    (goto _label_4))
  (:`Completed`
    (goto _label_4)))

(event `EnhancedInput|/Game/DekogonDrone01/Blueprints/Input/IA_LookUp`
  (params (ActionValue :type "Float (double-precision)") (ElapsedSeconds :type "Float (double-precision)") (TriggeredSeconds :type "Float (double-precision)") (InputAction :type "InputAction Object Reference" :default "/Game/DekogonDrone01/Blueprints/Input/IA_LookUp.IA_LookUp"))
  ;[1 1 1] Audio&Animation
  (:`Triggered`
    (`SceneComponent.K2_AddRelativeRotation` (`self.SpringArm`) (`KismetMathLibrary.MakeRotator` 0.0 (* ActionValue (`self.Vertical Camera Rotation`))) false false :!label _label_5))
  (:`Started`
    (goto _label_5))
  (:`Completed`
    (goto _label_5)))

(event `EnhancedInput|/Game/DekogonDrone01/Blueprints/Input/IA_LookRight`
  (params (ActionValue :type "Float (double-precision)") (ElapsedSeconds :type "Float (double-precision)") (TriggeredSeconds :type "Float (double-precision)") (InputAction :type "InputAction Object Reference" :default "/Game/DekogonDrone01/Blueprints/Input/IA_LookRight.IA_LookRight"))
  (bind _lookright (`self.LookRight`))
  ;[1 1 1] Audio&Animation
  (:`Triggered`
    (bind _output_get (set `self.LookRight` ActionValue :!label _label_6))
    (set `self.MouseRot` (`KismetMathLibrary.SelectFloat` (`KismetMathLibrary.SelectFloat` (`KismetMathLibrary.SelectFloat` (`KismetMathLibrary.SelectFloat` (`KismetMathLibrary.SelectFloat` (`KismetMathLibrary.SelectFloat` (`KismetMathLibrary.SelectFloat` 0.7 0.6 (> _lookright 0.6)) 0.4 (> _lookright 0.5)) 0.4 (> _lookright 0.4)) 0.3 (> _lookright 0.3)) 0.2 (> _lookright 0.2)) 0.1 (> _lookright 0.1)) (`KismetMathLibrary.SelectFloat` (`KismetMathLibrary.SelectFloat` (`KismetMathLibrary.SelectFloat` (`KismetMathLibrary.SelectFloat` (`KismetMathLibrary.SelectFloat` (`KismetMathLibrary.SelectFloat` (`KismetMathLibrary.SelectFloat` -0.7 -0.6 (< _lookright -0.6)) -0.5 (< _lookright -0.5)) -0.4 (< _lookright -0.4)) -0.3 (< _lookright -0.3)) -0.2 (< _lookright -0.2)) -0.1 (< _lookright -0.1)) 0.0 (< _lookright 0.0)) (> _lookright 0.0))))
  (:`Started`
    (goto _label_6))
  (:`Completed`
    (goto _label_6)))

(fn `UserConstructionScript`
  (bind _sm_turret02 (`self.SM_Turret02`))
  (bind _dekogondrone (`self.DekogonDrone`))
  (bind _returnvalue (`KismetMathLibrary.Conv_IntToBool` (`self.TurretType`)))
  (`SceneComponent.SetVisibility` (`self.SM_Turret01`) _returnvalue false)
  (`SceneComponent.SetVisibility` _sm_turret02 (not _returnvalue) false)
  (`PrimitiveComponent.SetMaterial` _dekogondrone 0 (`self.Drone Material`))
  (`MeshComponent.SetScalarParameterValueOnMaterials` _sm_turret02 "Emmisive Strength" (`self.Emmisive Strength`))
  (`MeshComponent.SetScalarParameterValueOnMaterials` (`self.SM_Turret01`) "Emmisive Strength" (`self.Emmisive Strength`))
  (`MeshComponent.SetScalarParameterValueOnMaterials` _dekogondrone "Emmisive Strength" (`self.Emmisive Strength`))
  (`MeshComponent.SetVectorParameterValueOnMaterials` _dekogondrone "Base Color" (`KismetMathLibrary.Conv_LinearColorToVector` (`self.Base Color`)))
  (`MeshComponent.SetVectorParameterValueOnMaterials` (`self.SM_Turret01`) "Base Color" (`KismetMathLibrary.Conv_LinearColorToVector` (`self.Base Color`)))
  (`MeshComponent.SetVectorParameterValueOnMaterials` _sm_turret02 "Base Color" (`KismetMathLibrary.Conv_LinearColorToVector` (`self.Base Color`)))
  (`MeshComponent.SetVectorParameterValueOnMaterials` _dekogondrone "Emmisive Color Turret 01" (`KismetMathLibrary.Conv_LinearColorToVector` (`self.Emmisive Color Turret 01`)))
  (`MeshComponent.SetVectorParameterValueOnMaterials` (`self.SM_Turret01`) "Emmisive Color Turret 01" (`KismetMathLibrary.Conv_LinearColorToVector` (`self.Emmisive Color Turret 01`)))
  (`MeshComponent.SetVectorParameterValueOnMaterials` _sm_turret02 "Emmisive Color Turret 01" (`KismetMathLibrary.Conv_LinearColorToVector` (`self.Emmisive Color Turret 01`)))
  (`MeshComponent.SetVectorParameterValueOnMaterials` _dekogondrone "Emmisive Color Thrusters" (`KismetMathLibrary.Conv_LinearColorToVector` (`self.Emmisive Color Thrusters`)))
  (`MeshComponent.SetVectorParameterValueOnMaterials` (`self.SM_Turret01`) "Emmisive Color Thrusters" (`KismetMathLibrary.Conv_LinearColorToVector` (`self.Emmisive Color Thrusters`)))
  (`MeshComponent.SetVectorParameterValueOnMaterials` _sm_turret02 "Emmisive Color Thrusters" (`KismetMathLibrary.Conv_LinearColorToVector` (`self.Emmisive Color Thrusters`)))
  (`MeshComponent.SetVectorParameterValueOnMaterials` _dekogondrone "Emmisive Color Turret 02" (`KismetMathLibrary.Conv_LinearColorToVector` (`self.Emmisive Color Turret 02`)))
  (`MeshComponent.SetVectorParameterValueOnMaterials` (`self.SM_Turret01`) "Emmisive Color Turret 02" (`KismetMathLibrary.Conv_LinearColorToVector` (`self.Emmisive Color Turret 02`)))
  (`MeshComponent.SetVectorParameterValueOnMaterials` _sm_turret02 "Emmisive Color Turret 02" (`KismetMathLibrary.Conv_LinearColorToVector` (`self.Emmisive Color Turret 02`))))